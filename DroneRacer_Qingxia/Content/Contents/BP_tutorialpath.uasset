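; Tutorial camera path actor that moves a CameraActor tagged TutorialCam along its spline, one point at a time.
; A gameplay message on the tutorial menu channel sets the current point index from its IntVector payload and starts a timeline.
; The timeline interpolates spline distance to the next point, placing the camera there and facing it along the spline tangent.
; Tick looks up the tagged camera whenever the reference is invalid.
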(event `self.ReceiveBeginPlay`
  (bind (_asynctaskproxy _actualchannel _payload) (`|AsyncAction_ListenForGameplayMessages` (struct :`TagName` "UI.Layer.GameMenu.Tutorial") "/Script/CoreUObject.IntVector")
    (:`OnMessageReceived`
      (set `self.CurrentIndex` (`.X` (break `IntVector` _payload)))
      (`self.MoveToNext`))))

(event `self.ReceiveTick`
  (params (DeltaSeconds :type "Float (single-precision)"))
  (`self.MoveActor`
    (:`then`)
    (:`else`
      (bind _outactors (`GameplayStatics.GetAllActorsOfClassWithTag` "/Script/Engine.CameraActor" "TutorialCam"))
      (set `self.MoveActor` (`|GetArrayItem` _outactors)))))

(event `MoveToNext`
  (bind _spline (`self.Spline`))
  (bind _currentindex (`self.CurrentIndex`))
  (bind _spline_2 (`self.Spline`))
  (bind _returnvalue (- (`SplineComponent.GetNumberOfSplinePoints` _spline) 1))
  (bind (_direction _splinepos) (`Timeline|Timeline` :!via `PlayFromStart`)
    (:`Update`
      (bind _returnvalue_2 (`KismetMathLibrary.Lerp` (`SplineComponent.GetDistanceAlongSplineAtSplinePoint` _spline (`KismetMathLibrary.Clamp` _currentindex 0 _returnvalue)) (`SplineComponent.GetDistanceAlongSplineAtSplinePoint` _spline (`KismetMathLibrary.Clamp` (+ _currentindex 1) 0 _returnvalue)) _splinepos))
      (`self.K2_SetActorLocationAndRotation` (`self.MoveActor`) (`SplineComponent.GetLocationAtDistanceAlongSpline` _spline_2 _returnvalue_2 "World") (`KismetMathLibrary.Conv_VectorToRotator` (`SplineComponent.GetTangentAtDistanceAlongSpline` _spline_2 _returnvalue_2 "World")) false false))))

(fn `UserConstructionScript`)